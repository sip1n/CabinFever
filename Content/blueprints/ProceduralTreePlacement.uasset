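; Procedural placement actor that scatters static mesh components, trees by its name, around its origin.
; The construction script loops ObjectCount times, placing each mesh at a random unit vector scaled by DistanceX and DistanceY and flattened to zero height.
; Each instance gets random yaw and independent per-axis scale between MinScale and MaxScale.
; The randomness is unseeded, so layouts change whenever construction reruns.
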(event EventBeginPlay)

(event Collision|EventActorBeginOverlap
  (params (OtherActor :type Actor%20Object%20Reference)))

(event EventTick
  (params (DeltaSeconds :type Float%20%28single-precision%29)))

(fn ConstructionScript
  (bind _minscale (Variables|Default|GetMinScale))
  (bind _maxscale (Variables|Default|GetMaxScale))
  (bind _returnvalue (Math|Random|RandomFloatinRange _minscale _maxscale))
  ;[1 0 0.8542] ForLoop
  (for _index (range 1 (Variables|Default|GetObjectCount))
    (AddComponent|AddStaticMeshComponent false (Math|Transform|MakeTransform (* (Math|Random|RandomUnitVector) (Math|Vector|MakeVector (Variables|Default|GetDistanceX) (Variables|Default|GetDistanceY) 0.0)) (Math|Rotator|MakeRotator 0.0 0.0 (Math|Random|RandomFloatinRange 0.0 999999.0)) (Math|Vector|MakeVector _returnvalue _returnvalue _returnvalue)))))